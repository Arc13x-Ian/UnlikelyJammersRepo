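; BP_ScuffedAsHellLevelLoaderSecond is a trigger box that loads a level once enough players have entered it.
; A Box overlap by a first-person character's capsule increments a player count, which is never decremented on exit.
; When the count equals the target player number, it finds the UI_Handler actor and calls LoadLevel with either the Theater level, if PlayMovie is set, or the configured level name.
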(event OnComponentBeginOverlap(Box)
  (params (OverlappedComponent :type Primitive%20Component%20Object%20Reference) (OtherActor :type Actor%20Object%20Reference) (OtherComp :type Primitive%20Component%20Object%20Reference) (OtherBodyIndex :type Integer) (bFromSweep :type Boolean) (SweepResult :type Hit%20Result%20Structure%20%28by%20ref%29))
  (bind _howmanyplayer (Variables|Default|GetHowManyPlayer))
  (bind _asbp_first_person_character (Utilities|Casting|CastToBP_FirstPersonCharacter OtherActor))
  (if (== OtherComp (Variables|/Script/Engine.Character|GetCapsuleComponent _asbp_first_person_character))
    (Math|Integer|IncrementInt _howmanyplayer
      (:%20%20
        (Development|PrintString "Increment player count")
        (if (== (Variables|Default|GetTargetPlayer) _howmanyplayer)
          (bind _returnvalue (Actor|GetActorOfClass "/Game/UI/Blueprints/UI_Handler.UI_Handler_C"))
          (if (Variables|Default|GetPlayMovie?)
            (Default|LoadLevel _returnvalue "Theater")
            (else
              (Default|LoadLevel _returnvalue (Variables|Default|GetLevel%20Name)))))))))

(event EventBeginPlay)

(event Collision|EventActorBeginOverlap
  (params (OtherActor :type Actor%20Object%20Reference)))

(event EventTick
  (params (DeltaSeconds :type Float%20%28single-precision%29)))

(fn ConstructionScript)