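; BP_Combiner is an actor that absorbs overlapping PreceptionObjects with a matching combine channel, showing a red, green, blue or yellow piece in their place.
; Construction removes unused color slots; BeginPlay caches attach-point locations, shrinks pieces to zero scale under Origin, and optionally adds a "Grab" tag.
; An ObjectChecker match moves that color's piece to its cached location at full scale, then tags the incoming object "Deleting" and destroys it next tick.
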(event OnComponentBeginOverlap(ObjectChecker)
  (params (OverlappedComponent :type Primitive%20Component%20Object%20Reference) (OtherActor :type Actor%20Object%20Reference) (OtherComp :type Primitive%20Component%20Object%20Reference) (OtherBodyIndex :type Integer) (bFromSweep :type Boolean) (SweepResult :type Hit%20Result%20Structure%20%28by%20ref%29))
  (bind _greenattachobject (Variables|Default|GetGreenAttachObject))
  (bind _redattachobject (Variables|Default|GetRedAttachObject))
  (bind _yellowattachobject (Variables|Default|GetYellowAttachObject))
  (bind _blueattachobject (Variables|Default|GetBlueAttachObject))
  (bind _aspreception_object (Utilities|Casting|CastToPreceptionObject OtherActor))
  (Development|PrintString (Utilities|String|ToString(Boolean) (== (Variables|/Game/PreceptionBox_Blueprints/PreceptionObject.PreceptionObject_C|GetCombineChannel _aspreception_object) (Variables|Default|GetChannel))))
  (if (== (Variables|/Game/PreceptionBox_Blueprints/PreceptionObject.PreceptionObject_C|GetCombineChannel _aspreception_object) (Variables|Default|GetChannel))
    (Utilities|FlowControl|Sequence
      (:then_0
        (switch Utilities|FlowControl|Switch|SwitchonColors (Variables|/Game/PreceptionBox_Blueprints/PreceptionObject.PreceptionObject_C|GetColor _aspreception_object)
          (:NewEnumerator0
            (Transformation|SetRelativeLocation _redattachobject (Variables|Default|GetRed%20Relative%20Location) false false)
            (Transformation|SetRelativeScale3D _redattachobject "1.000000,1.000000,1.000000"))
          (:NewEnumerator1
            (Transformation|SetRelativeLocation _greenattachobject (Variables|Default|GetGreen%20Relative%20Location) false false)
            (Transformation|SetRelativeScale3D _greenattachobject "1.000000,1.000000,1.000000"))
          (:NewEnumerator2
            (Transformation|SetRelativeLocation _blueattachobject (Variables|Default|GetBlue%20Relative%20Location) false false)
            (Transformation|SetRelativeScale3D _blueattachobject "1.000000,1.000000,1.000000"))
          (:NewEnumerator3
            (Transformation|SetRelativeLocation _yellowattachobject (Variables|Default|GetYellow%20Relative%20Location) false false)
            (Transformation|SetRelativeScale3D _yellowattachobject "1.000000,1.000000,1.000000"))))
      (:then_1
        (Utilities|Array|AddUnique (Variables|/Script/Engine.Actor|GetTags _aspreception_object) "Deleting")
        (Utilities|FlowControl|DelayUntilNextTick)
        (Actor|DestroyActor _aspreception_object)))))

(event Collision|EventActorBeginOverlap
  (params (OtherActor :type Actor%20Object%20Reference)))

(event EventTick
  (params (DeltaSeconds :type Float%20%28single-precision%29)))

(event EventBeginPlay
  (bind _redattachobject (Variables|Default|GetRedAttachObject))
  (bind _blueattachobject (Variables|Default|GetBlueAttachObject))
  (bind _yellowattachobject (Variables|Default|GetYellowAttachObject))
  (bind _greenattachobject (Variables|Default|GetGreenAttachObject))
  (Utilities|FlowControl|Sequence
    (:then_0
      (Utilities|FlowControl|Sequence
        (:then_0
          (bind _redattachpoint (Variables|Points|GetRedAttachPoint)
            (:then
              (Variables|Default|SetRed%20Relative%20Location (Variables|/Script/Engine.SceneComponent|GetRelativeLocation _redattachpoint))
              (Transformation|SetRelativeLocation _redattachpoint "0, 0, 0" false true)
              (Transformation|SetRelativeScale3D _redattachobject "0, 0, 0")
              (Rendering|SetVisibility _redattachobject true false)
              (Transformation|AttachComponentToComponent _redattachobject (Variables|Default|GetOrigin) "None" "KeepWorld" "KeepWorld" "KeepRelative" true))
            (:else)))
        (:then_1
          (bind _blueattachpoint (Variables|Points|GetBlueAttachPoint)
            (:then
              (Variables|Default|SetBlue%20Relative%20Location (Variables|/Script/Engine.SceneComponent|GetRelativeLocation _blueattachpoint))
              (Transformation|SetRelativeLocation _blueattachpoint "0, 0, 0" false true)
              (Transformation|SetRelativeScale3D _blueattachobject "0, 0, 0")
              (Rendering|SetVisibility _blueattachobject true false)
              (Transformation|AttachComponentToComponent _blueattachobject (Variables|Default|GetOrigin) "None" "KeepWorld" "KeepWorld" "KeepRelative" true))
            (:else)))
        (:then_2
          (bind _yellowattachpoint (Variables|Points|GetYellowAttachPoint)
            (:then
              (Variables|Default|SetYellow%20Relative%20Location (Variables|/Script/Engine.SceneComponent|GetRelativeLocation _yellowattachpoint))
              (Transformation|SetRelativeLocation _yellowattachpoint "0, 0, 0" false true)
              (Transformation|SetRelativeScale3D _yellowattachobject "0, 0, 0")
              (Rendering|SetVisibility _yellowattachobject true false)
              (Transformation|AttachComponentToComponent _yellowattachobject (Variables|Default|GetOrigin) "None" "KeepWorld" "KeepWorld" "KeepRelative" true))
            (:else)))
        (:then_3
          (bind _greenattachpoint (Variables|Points|GetGreenAttachPoint)
            (:then
              (Variables|Default|SetGreen%20Relative%20Location (Variables|/Script/Engine.SceneComponent|GetRelativeLocation _greenattachpoint))
              (Transformation|SetRelativeLocation _greenattachpoint "0, 0, 0" false true)
              (Transformation|SetRelativeScale3D _greenattachobject "0.000000,0.000000,0.000000")
              (Rendering|SetVisibility _greenattachobject true false)
              (Transformation|AttachComponentToComponent _greenattachobject (Variables|Default|GetOrigin) "None" "KeepWorld" "KeepWorld" "KeepRelative" true))
            (:else)))))
    (:then_1
      (if (Variables|Default|GetGrabbable?)
        (Utilities|Array|AddUnique (Variables|Actor|GetTags) "Grab")))))

(fn ConstructionScript
  (Utilities|FlowControl|Sequence
    (:then_0
      (Utilities|FlowControl|Sequence
        (:then_0
          (if (not (Variables|Default|GetHasRedAttach?))
            (Components|DestroyComponent (Variables|Default|GetRedAttachObject))
            (Components|DestroyComponent (Variables|Points|GetRedAttachPoint))))
        (:then_1
          (if (not (Variables|Default|GetHasBlueAttach?))
            (Components|DestroyComponent (Variables|Default|GetBlueAttachObject))
            (Components|DestroyComponent (Variables|Points|GetBlueAttachPoint))))
        (:then_2
          (if (not (Variables|Default|GetHasYellowAttach?))
            (Components|DestroyComponent (Variables|Default|GetYellowAttachObject))
            (Components|DestroyComponent (Variables|Points|GetYellowAttachPoint))))
        (:then_3
          (if (not (Variables|Default|GetHasGreenAttach?))
            (Components|DestroyComponent (Variables|Default|GetGreenAttachObject))
            (Components|DestroyComponent (Variables|Points|GetGreenAttachPoint))))))))