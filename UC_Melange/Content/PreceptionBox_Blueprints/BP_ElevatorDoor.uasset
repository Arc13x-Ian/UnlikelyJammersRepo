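; Sliding double elevator door that either opens automatically at level start or, as an end-level door, waits for three color signals.
; A timeline eases both panels from their initial positions to stop markers, firing a 2D sound on every update.
; TalktoDoor flip-flops Red, Blue and Yellow readiness per call, opening the doors once all three are ready.
; Nothing here closes the doors again.
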(event Custom|OpenDoors
  (bind _alpha (Timeline|DoorTimeline Play)
    (:Update
      (Utilities|FlowControl|Sequence
        (:then_0
          (Transformation|SetWorldLocation (Variables|Default|GetDoor_R) (Math|Interpolation|Ease "EaseInOut" _alpha (Variables|Default|GetDoor_RIntialLocation) (Transformation|GetWorldLocation (Variables|Default|GetDoor_R_Stop)) 3.0) false true))
        (:then_1
          (Transformation|SetWorldLocation (Variables|Default|GetDoor_L) (Math|Interpolation|Ease "EaseInOut" _alpha (Variables|Default|GetDoor_LIntialLocation) (Transformation|GetWorldLocation (Variables|Default|GetDoor_L_Stop)) 3.0) false true))
        (:then_2
          (Audio|PlaySound2D (Variables|Default|GetSound) 1.0 1.0 0.0 0 0))))))

(event EventBeginPlay
  (Variables|Default|SetDoor_RIntialLocation (Transformation|GetWorldLocation (Variables|Default|GetDoor_R)))
  (Variables|Default|SetDoor_LIntialLocation (Transformation|GetWorldLocation (Variables|Default|GetDoor_L)))
  (if (not (Variables|Default|GetEndLevelDoor?))
    (Utilities|FlowControl|Delay 2.0)
    (CallFunction|OpenDoors)))

(event Collision|EventActorBeginOverlap
  (params (OtherActor :type Actor%20Object%20Reference)))

(event EventTick
  (params (DeltaSeconds :type Float%20%28single-precision%29)))

(event EventTalktoDoor
  (params (Color :type Colors%20Enum :default "NewEnumerator0"))
  (if (Variables|Default|GetEndLevelDoor?)
    (switch Utilities|FlowControl|Switch|SwitchonColors Color
      (:NewEnumerator0
        (Utilities|FlowControl|FlipFlop
          (:A
            (Variables|Default|SetRedReady? true)
            (Development|PrintString "RED T")
            (if (and (Variables|Default|GetRedReady?) (and (Variables|Default|GetBlueReady?) (Variables|Default|GetYellowReady?))) :!label _label
              (CallFunction|OpenDoors)))
          (:B
            (Variables|Default|SetRedReady? false)
            (Development|PrintString "RED F"))))
      (:NewEnumerator2
        (Utilities|FlowControl|FlipFlop
          (:A
            (Variables|Default|SetBlueReady? true)
            (Development|PrintString "BLUE T")
            (goto _label))
          (:B
            (Variables|Default|SetBlueReady? false)
            (Development|PrintString "BLUE F"))))
      (:NewEnumerator3
        (Utilities|FlowControl|FlipFlop
          (:A
            (Variables|Default|SetYellowReady? true)
            (Development|PrintString "YELLOW T")
            (goto _label))
          (:B
            (Variables|Default|SetYellowReady? false)
            (Development|PrintString "YELLOW F")))))))

(fn ConstructionScript)