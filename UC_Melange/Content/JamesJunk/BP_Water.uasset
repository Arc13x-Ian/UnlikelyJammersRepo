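; BP_Water is a water actor that plays a one-time splash effect when something overlaps its box trigger.
; The NSSplash effect is switched off on BeginPlay, and a DoOnce on the box overlap activates it for the first overlap of any actor.
; After a short delay, it deactivates the splash and the DefaultSceneRoot component.
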(event OnComponentBeginOverlap(Box)
  (params (OverlappedComponent :type Primitive%20Component%20Object%20Reference) (OtherActor :type Actor%20Object%20Reference) (OtherComp :type Primitive%20Component%20Object%20Reference) (OtherBodyIndex :type Integer) (bFromSweep :type Boolean) (SweepResult :type Hit%20Result%20Structure%20%28by%20ref%29))
  (Utilities|FlowControl|DoOnce false
    (:Completed
      (Components|Activation|Activate (Variables|Default|GetNS_Splash) false)
      (Utilities|FlowControl|Delay 5.0)
      (Components|Activation|Deactivate (Variables|Default|GetNS_Splash))
      (Components|Activation|Deactivate (Variables|Default|GetDefaultSceneRoot)))))

(event EventBeginPlay
  (Components|Activation|Deactivate (Variables|Default|GetNS_Splash)))

(event Collision|EventActorBeginOverlap
  (params (OtherActor :type Actor%20Object%20Reference)))

(event EventTick
  (params (DeltaSeconds :type Float%20%28single-precision%29)))

(fn ConstructionScript)